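; BP_PitaController is the player controller that handles looking at, interacting with and carrying items.
; Each tick a short camera line trace finds actors with a BP_InteractableComponent and toggles hover as the target changes.
; IA_Grab forwards interact start and end to the hovered component.
; GrabItem attaches one actor at a time to the character's GrabLocation, and IA_Drop or DropAnyItem releases it.
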(event Input|EnhancedActionEvents|EnhancedInputActionIA_Grab
  (params (ActionValue :type Boolean) (ElapsedSeconds :type Float%20%28double-precision%29) (TriggeredSeconds :type Float%20%28double-precision%29) (InputAction :type Input%20Action%20Object%20Reference :default "/Game/FirstPerson/Input/Actions/IA_Grab.IA_Grab"))
  (bind _currentinteractablecomponent (Variables|Default|GetCurrentInteractableComponent))
  (bind _currentinteractablecomponent_2 (Variables|Default|GetCurrentInteractableComponent))
  (:Started
    (Utilities|IsValid _currentinteractablecomponent_2
      (:Is%20Valid
        (Default|InteractStart _currentinteractablecomponent_2))))
  (:Completed
    (Utilities|IsValid _currentinteractablecomponent
      (:Is%20Valid
        (Default|InteractEnd _currentinteractablecomponent)))))

(event Input|EnhancedActionEvents|EnhancedInputActionIA_Drop
  (params (ActionValue :type Boolean) (ElapsedSeconds :type Float%20%28double-precision%29) (TriggeredSeconds :type Float%20%28double-precision%29) (InputAction :type Input%20Action%20Object%20Reference :default "/Game/FirstPerson/Input/Actions/IA_Drop.IA_Drop"))
  (CallFunction|DropAnyItem))

(event EventBeginPlay
  (bind _asbp_pita_character (Utilities|Casting|CastToBP_PitaCharacter (Game|GetPlayerCharacter 0)))
  (Variables|Default|SetPitaCharacter _asbp_pita_character))

(event EventTick
  (params (DeltaSeconds :type Float%20%28single-precision%29))
  (bind _returnvalue (Game|GetPlayerCameraManager 0))
  (bind _returnvalue_2 (Transformation|GetActorLocation _returnvalue))
  (bind (_outhit _returnvalue_3) (Collision|LineTraceByChannel _returnvalue_2 (+ _returnvalue_2 (* (Transformation|GetActorForwardVector _returnvalue) 200)) "TraceTypeQuery1" false 0 "None"))
  (if _returnvalue_3
    (Utilities|IsValid (Actor|GetComponentbyClass (.hitactor _outhit) "/Game/PitaSimulator/InteractionSystem/BP_InteractableComponent.BP_InteractableComponent_C")
      (:Is%20Valid
        (Variables|Default|SetCurrentInteractableComponent (Actor|GetComponentbyClass (.hitactor _outhit) "/Game/PitaSimulator/InteractionSystem/BP_InteractableComponent.BP_InteractableComponent_C"))
        (Utilities|FlowControl|Sequence
          (:then_0
            (Utilities|IsValid (Variables|Default|GetLastInteractableComponent)
              (:Is%20Valid
                (if (not (== (Variables|Default|GetLastInteractableComponent) (Variables|Default|GetCurrentInteractableComponent)))
                  (Default|Unhover (Variables|Default|GetLastInteractableComponent))
                  (Default|Hover (Variables|Default|GetCurrentInteractableComponent))))
              (:Is%20Not%20Valid
                (Default|Hover (Variables|Default|GetCurrentInteractableComponent)))))
          (:then_1
            (Variables|Default|SetLastInteractableComponent (Variables|Default|GetCurrentInteractableComponent)))))
      (:Is%20Not%20Valid
        (Variables|Default|SetCurrentInteractableComponent 0 :!label _label)
        (Utilities|IsValid (Variables|Default|GetLastInteractableComponent)
          (:Is%20Valid
            (Default|Unhover (Variables|Default|GetLastInteractableComponent))
            (Variables|Default|SetLastInteractableComponent 0)))))
    (else
      (goto _label))))

(event EventDropAnyItem
  (Utilities|IsValid (Variables|Default|GetGrabbed%20Interactable%20Component)
    (:Is%20Valid
      (Default|Release (Variables|Default|GetGrabbed%20Interactable%20Component))
      (Variables|Default|SetGrabbed%20Interactable%20Component 0)
      (Variables|Default|SetGrabbed%20Actor 0)
      (Variables|Default|SetAlreadyGrabbed? false))))

(fn ConstructionScript)

(fn GetGrabbedItem
  (bind _grabbed_actor (Variables|Default|GetGrabbed%20Actor))
  (Utilities|IsValid _grabbed_actor
    (:Is%20Valid
      (return true _grabbed_actor))
    (:Is%20Not%20Valid
      (return false 0))))

(fn GrabItem
  (params (GrabbedInteractableComponent :type BP%20Interactable%20Component%20Object%20Reference) (GrabbedActor :type Actor%20Object%20Reference))
  (if (Variables|Default|GetAlreadyGrabbed?)
    (return false)
    (else
      (Variables|Default|SetGrabbed%20Interactable%20Component GrabbedInteractableComponent)
      (bind _output_get (Variables|Default|SetGrabbed%20Actor GrabbedActor))
      (bind _returnvalue (Transformation|AttachComponentToComponent _output_get (Variables|/Game/PitaSimulator/Player/BP_PitaCharacter.BP_PitaCharacter_C|GetGrabLocation (Variables|Default|GetPitaCharacter)) "None" "SnapToTarget" "SnapToTarget" "KeepRelative" false))
      (bind _output_get_2 (Variables|Default|SetAlreadyGrabbed? _returnvalue))
      (Variables|/Game/PitaSimulator/InteractionSystem/BP_InteractableComponent.BP_InteractableComponent_C|SetAlreadyGrabbed? (Variables|Default|GetGrabbed%20Interactable%20Component) true)
      (return _output_get_2))))