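; BP_PitaGameMode is the game mode for the pita simulator, holding the player's money and the bakery name.
; Events add money or remove it, clamping the balance at zero, and a getter returns the current amount.
; Renaming the bakery stores the new name and calls the OnBakeryNameChanged dispatcher so listeners can react.
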(event Custom|ChangeBakeryName
  (params (NewName :type Name))
  (bind _output_get (Variables|Default|SetBakeryName NewName))
  (Default|CallOnBakeryNameChanged _output_get))

(event EventBeginPlay)

(event EventTick
  (params (DeltaSeconds :type Float%20%28single-precision%29)))

(event EventAddMoney
  (params (Value :type Integer))
  (Variables|Default|SetMoney (+ (Variables|Default|GetMoney) Value)))

(event EventRemoveMoney
  (params (Value :type Integer))
  (if (> (Variables|Default|GetMoney) Value)
    (Variables|Default|SetMoney (- (Variables|Default|GetMoney) Value))
    (else
      (Variables|Default|SetMoney 0))))

(fn ConstructionScript
  (|CallParentFunction))

(fn GetCurrentMoney
  (return (Variables|Default|GetMoney)))