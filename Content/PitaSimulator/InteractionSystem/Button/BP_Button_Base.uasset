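; Base interactable button actor that toggles between Closed and Opened states when used.
; When its interactable component fires OnInteractStart, it flips the state, while a Broken button stays Broken.
; It then swaps the static mesh material to match the state and broadcasts the state through the OnButtonInteraction dispatcher.
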(event OnInteractStart(BP_InteractableComponent)
  (bind _output_get (Variables|Default|SetState (Utilities|Select :Index (Variables|Default|GetState) :NewEnumerator0 "NewEnumerator1" :NewEnumerator1 "NewEnumerator0" :NewEnumerator2 "NewEnumerator2")))
  (Rendering|Material|SetMaterial (Variables|Default|GetStaticMesh) 0 (Utilities|Select :Index _output_get :NewEnumerator0 "/Engine/MapTemplates/Materials/BasicAsset02.BasicAsset02" :NewEnumerator1 "/AnimationSharing/AnimSharingGreen.AnimSharingGreen" :NewEnumerator2 "/Engine/EngineMeshes/BackgroundMaterial.BackgroundMaterial"))
  (Default|CallOnButtonInteraction (Variables|Default|GetState)))

(event EventBeginPlay
  (|CallParentFunction))

(event Collision|EventActorBeginOverlap
  (params (OtherActor :type Actor%20Object%20Reference))
  (|CallParentFunction OtherActor) ; This node is disabled and will not be called.\nDrag off pins to build functionality.
)

(event EventTick
  (params (DeltaSeconds :type Float%20%28single-precision%29))
  (|CallParentFunction DeltaSeconds) ; This node is disabled and will not be called.\nDrag off pins to build functionality.
)

(fn ConstructionScript
  (|CallParentFunction))