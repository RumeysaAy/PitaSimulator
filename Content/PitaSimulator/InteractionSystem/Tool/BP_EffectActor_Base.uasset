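; Base effect actor that a player works on with a grabbed item of a specific interaction type, then is destroyed on completion.
; Interactable component events drive a timeline, rate-matched to the interaction duration, whose alpha sets Progress and uniform mesh scale.
; Ending interaction stops the timeline so it can resume from partial progress, while a process restart resets Progress and scale to full.
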(event OnInteractEnd(BP_InteractableComponent)
  (Development|PrintString "Intreact ended")
  (bind _alpha (Timeline|ProgressTimeline Stop)
    (:Update
      (bind _output_get (Variables|Default|SetProgress _alpha))
      (Transformation|SetWorldScale3D (Variables|Default|GetStaticMesh) (Math|Conversions|ToVector(Float) _output_get)))))

(event OnInteractionCompleted(BP_InteractableComponent)
  (Actor|DestroyActor))

(event OnProcessRestart(BP_InteractableComponent)
  (Variables|Default|SetProgress 1.0)
  (Transformation|SetWorldScale3D (Variables|Default|GetStaticMesh) "1.000000,1.000000,1.000000"))

(event OnInteractStart(BP_InteractableComponent)
  (bind (_grabbed _grabbedactor) (Class|BPIInteractionSystem|GetGrabbedItem(Message) (Game|GetPlayerController 0)))
  (if _grabbed
    (if (Utilities|Enum|Equal(Enum) (Variables|/Game/PitaSimulator/InteractionSystem/BP_InteractableComponent.BP_InteractableComponent_C|GetInteractionType (Actor|GetComponentbyClass _grabbedactor "/Game/PitaSimulator/InteractionSystem/BP_InteractableComponent.BP_InteractableComponent_C")) "NewEnumerator2")
      (Default|TryStartInteractionProcess (Variables|Default|GetBP_InteractableComponent))
      (Development|PrintString "Intreact started")
      (Components|Timeline|SetPlayRate (Variables|Default|GetProgressTimeline) (/ 1 (Variables|/Game/PitaSimulator/InteractionSystem/BP_InteractableComponent.BP_InteractableComponent_C|GetInteractionDuration (Variables|Default|GetBP_InteractableComponent))))
      (if (!= (Variables|Default|GetProgress) 1.0)
        (bind _alpha (Timeline|ProgressTimeline Play)
          (:Update
            (bind _output_get (Variables|Default|SetProgress _alpha))
            (Transformation|SetWorldScale3D (Variables|Default|GetStaticMesh) (Math|Conversions|ToVector(Float) _output_get))))
        (else
          (Timeline|ProgressTimeline PlayFromStart))))))

(event EventBeginPlay
  (|CallParentFunction) ; This node is disabled and will not be called.\nDrag off pins to build functionality.
)

(event Collision|EventActorBeginOverlap
  (params (OtherActor :type Actor%20Object%20Reference))
  (|CallParentFunction OtherActor) ; This node is disabled and will not be called.\nDrag off pins to build functionality.
)

(event EventTick
  (params (DeltaSeconds :type Float%20%28single-precision%29))
  (|CallParentFunction DeltaSeconds) ; This node is disabled and will not be called.\nDrag off pins to build functionality.
)

(fn ConstructionScript
  (|CallParentFunction))