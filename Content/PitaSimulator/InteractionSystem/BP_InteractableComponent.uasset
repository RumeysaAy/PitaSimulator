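; Actor component that makes its owner interactable, relaying hover, grab, release and interaction events through dispatchers.
; Start and end branch on interaction type: Grab and Tool are picked up and released, Interaction runs timed progress, and Effect requires a held Tool.
; A timer drives completion, pausing on interrupt and then resuming or restarting according to the end policy.
; SnapToSlot requests physics disabling and attaches the owner to a slot actor.
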(event EventBeginPlay)

(event EventTick
  (params (DeltaSeconds :type Float%20%28single-precision%29)))

(fn Hover
  (Development|PrintString (Utilities|String|Append "Hovered interactable actor:" (Utilities|GetDisplayName (Components|GetOwner))) true true "(R=0.000000,G=1.000000,B=0.061501,A=1.000000)" 1.0 "InteractionHover")
  (Default|CallOnHover))

(fn Unhover
  (if (Variables|Default|GetInteractionStarted)
    (CallFunction|InteractEnd))
  (Development|PrintString (Utilities|String|Append "UnHovered interactable actor:" (Utilities|GetDisplayName (Components|GetOwner))) true true "(R=1.000000,G=0.000000,B=0.075129,A=1.000000)" 1.0 "InteractionUnHover")
  (Default|CallOnUnhover))

(fn InteractStart
  (switch Utilities|FlowControl|Switch|SwitchonEInteractionType (Variables|Default|GetInteractionType)
    (:NewEnumerator0
      (Default|CallOnGrab :!label _label))
    (:NewEnumerator1
      (Default|CallOnInteractStart)
      (CallFunction|TryStartInteractionProcess))
    (:NewEnumerator2
      (goto _label))
    (:NewEnumerator4
      (bind (_grabbed _grabbedactor) (Class|BPIInteractionSystem|GetGrabbedItem(Message) (Game|GetPlayerController 0)))
      (if _grabbed
        (if (Utilities|Enum|Equal(Enum) (Variables|BP_InteractableComponent_C|GetInteractionType (Actor|GetComponentbyClass _grabbedactor "BP_InteractableComponent_C")) "NewEnumerator2")
          (Default|CallOnInteractStart)
          (CallFunction|TryStartInteractionProcess))))))

(fn InteractEnd
  (bind _interactioncompletationtimer (Variables|Process|GetInteractionCompletationTimer))
  (switch Utilities|FlowControl|Switch|SwitchonEInteractionType (Variables|Default|GetInteractionType)
    (:NewEnumerator0
      (if (Variables|Default|GetAlreadyGrabbed?) :!label _label
        (CallFunction|Release)))
    (:NewEnumerator1
      (Default|CallOnInteractEnd :!label _label_2)
      (if (Utilities|Time|IsTimerActivebyHandle _interactioncompletationtimer)
        (Utilities|Time|PauseTimerbyHandle _interactioncompletationtimer)
        (Development|PrintString "Interaction Paused")
        (if (Utilities|Enum|Equal(Enum) (Variables|Process|GetInteractionEndPolicy) "NewEnumerator0")
          (Default|CallOnProcessRestart))))
    (:NewEnumerator2
      (goto _label))
    (:NewEnumerator4
      (if (Variables|Default|GetInteractionStarted)
        (Variables|Default|SetInteractionStarted false)
        (goto _label_2)))))

(fn Release
  (Variables|Default|SetAlreadyGrabbed? false)
  (Default|CallOnRelease))

(fn InteractCompleted
  (Utilities|Time|ClearandInvalidateTimerbyHandle (Variables|Process|GetInteractionCompletationTimer))
  (Development|PrintString "InteractionCompleted")
  (Default|CallOnInteractionCompleted))

(fn SnaptoSlot
  (params (ItemSlot :type BP%20Item%20Slot%20Base%20Object%20Reference))
  (Default|CallOnPhysicsDisable)
  (Transformation|AttachActorToActor (Components|GetOwner) ItemSlot "None" "SnapToTarget" "SnapToTarget" "KeepRelative" false))

(fn TryStartInteractionProcess
  (if (Math|Boolean|ANDBoolean (Utilities|Time|IsValidTimerHandle (Variables|Process|GetInteractionCompletationTimer)) (Utilities|Enum|Equal(Enum) (Variables|Process|GetInteractionEndPolicy) "NewEnumerator1") (!= (Variables|Process|GetInteractionDuration) 0.0))
    (Variables|Default|SetInteractionStarted true)
    (Utilities|Time|UnpauseTimerbyHandle (Variables|Process|GetInteractionCompletationTimer))
    (else
      (Variables|Default|SetInteractionStarted true)
      (Development|PrintString "Progress started")
      (bind _returnvalue (Utilities|Time|SetTimerbyFunctionName 0 "InteractCompleted" (Variables|Process|GetInteractionDuration)))
      (Variables|Process|SetInteractionCompletationTimer _returnvalue))))