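; BP_ProcessActor_Base is a base actor for timed, interactable processes that shows progress through the color of its static mesh.
; Interaction events from BP_InteractableComponent start or resume a timeline, rate-scaled by InteractionDuration, and stop it when interaction ends.
; The timeline updates Progress and the Color parameter of a dynamic material created at BeginPlay.
; Process restart resets both progress and color, while completion only prints a debug message.
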(event OnInteractEnd(BP_InteractableComponent)
  (Development|PrintString "Intreact ended")
  (bind (_direction _alpha _color) (Timeline|ProgressTimeline Stop)
    (:Update
      (Variables|Default|SetProgress _alpha)
      (Rendering|Material|SetVectorParameterValue (Variables|Default|GetProgressMaterial) "Color" _color :!class /Script/Engine.MaterialInstanceDynamic))))

(event OnInteractStart(BP_InteractableComponent)
  (Development|PrintString "Intreact started")
  (Components|Timeline|SetPlayRate (Variables|Default|GetProgressTimeline) (/ 1 (Variables|/Game/PitaSimulator/InteractionSystem/BP_InteractableComponent.BP_InteractableComponent_C|GetInteractionDuration (Variables|Default|GetBP_InteractableComponent))))
  (if (!= (Variables|Default|GetProgress) 0.0)
    (bind (_direction _alpha _color) (Timeline|ProgressTimeline Play)
      (:Update
        (Variables|Default|SetProgress _alpha)
        (Rendering|Material|SetVectorParameterValue (Variables|Default|GetProgressMaterial) "Color" _color :!class /Script/Engine.MaterialInstanceDynamic)))
    (else
      (Timeline|ProgressTimeline PlayFromStart))))

(event OnInteractionCompleted(BP_InteractableComponent)
  (Development|PrintString "Intreact completed"))

(event OnProcessRestart(BP_InteractableComponent)
  (Rendering|Material|SetVectorParameterValue (Variables|Default|GetProgressMaterial) "Color" "(R=0.989583,G=0.989583,B=0.989583,A=1.000000)" :!class /Script/Engine.MaterialInstanceDynamic)
  (Variables|Default|SetProgress 0.0))

(event EventBeginPlay
  (|CallParentFunction)
  (bind _returnvalue (Rendering|Material|CreateDynamicMaterialInstance (Variables|Default|GetStaticMesh) 0 "/Game/PitaSimulator/InteractionSystem/Process/MI_ProgressMaterial.MI_ProgressMaterial" "None" :!class /Script/Engine.PrimitiveComponent))
  (Variables|Default|SetProgressMaterial _returnvalue))

(event Collision|EventActorBeginOverlap
  (params (OtherActor :type Actor%20Object%20Reference))
  (|CallParentFunction OtherActor) ; This node is disabled and will not be called.\nDrag off pins to build functionality.
)

(event EventTick
  (params (DeltaSeconds :type Float%20%28single-precision%29))
  (|CallParentFunction DeltaSeconds) ; This node is disabled and will not be called.\nDrag off pins to build functionality.
)

(fn ConstructionScript
  (|CallParentFunction))