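; BP_ItemSlot_Base is a base interactable slot that takes the player's held item and hands it back.
; When unlocked, interaction snaps a held actor into the slot if its class is in AttachableClass, then FindNewLockStatus locks the slot.
; When locked, an empty-handed player grabs the stored actor and frees the slot.
; Grab and drop go through PlayerController messages, while snapping and physics calls use the item's BP_InteractableComponent.
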(event OnInteractStart(BP_InteractableComponent)
  (if (Variables|Default|GetLocked?)
    (bind _grabbed (Class|BPIInteractionSystem|GetGrabbedItem(Message) (Game|GetPlayerController 0)))
    (if (not _grabbed)
      (Utilities|IsValid (Variables|Default|GetGrabbed%20Actor)
        (:Is%20Valid
          (Class|BPIInteractionSystem|GrabItem(Message) (Game|GetPlayerController 0) (Actor|GetComponentbyClass (Variables|Default|GetGrabbed%20Actor) "/Game/PitaSimulator/InteractionSystem/BP_InteractableComponent.BP_InteractableComponent_C") (Variables|Default|GetGrabbed%20Actor))
          (Default|CallOnPhysicsDisable (Actor|GetComponentbyClass (Variables|Default|GetGrabbed%20Actor) "/Game/PitaSimulator/InteractionSystem/BP_InteractableComponent.BP_InteractableComponent_C"))
          (Utilities|Array|RemoveItem (Variables|Default|GetAttachedActors) (Variables|Default|GetGrabbed%20Actor))
          (Variables|Default|SetLocked? false)
          (Variables|Default|SetGrabbed%20Actor 0))))
    (else
      (bind (_grabbed_2 _grabbedactor) (Class|BPIInteractionSystem|GetGrabbedItem(Message) (Game|GetPlayerController 0)))
      (bind _output_get (Variables|Default|SetGrabbed%20Actor _grabbedactor))
      (if (CallFunction|CheckAttachable? _grabbed_2 _output_get)
        (Class|BPIInteractionSystem|DropAnyItem(Message) (Game|GetPlayerController 0))
        (Default|SnaptoSlot (Actor|GetComponentbyClass (Variables|Default|GetGrabbed%20Actor) "/Game/PitaSimulator/InteractionSystem/BP_InteractableComponent.BP_InteractableComponent_C") self)
        (Utilities|Array|AddUnique (Variables|Default|GetAttachedActors) (Variables|Default|GetGrabbed%20Actor))
        (CallFunction|FindNewLockStatus)))))

(event EventBeginPlay
  (|CallParentFunction) ; This node is disabled and will not be called.\nDrag off pins to build functionality.
)

(event Collision|EventActorBeginOverlap
  (params (OtherActor :type Actor%20Object%20Reference))
  (|CallParentFunction OtherActor) ; This node is disabled and will not be called.\nDrag off pins to build functionality.
)

(event EventTick
  (params (DeltaSeconds :type Float%20%28single-precision%29))
  (|CallParentFunction DeltaSeconds) ; This node is disabled and will not be called.\nDrag off pins to build functionality.
)

(fn ConstructionScript
  (|CallParentFunction))

(fn CheckAttachable?
  (params (A :type Boolean) (Object :type Object%20Object%20Reference))
  (bind _asbp_interact_actor_base (Utilities|Casting|CastToBP_InteractActor_BaseClass (Utilities|GetClass Object))
    (:then
      (return (Math|Boolean|ANDBoolean A (!= (Utilities|Array|FindItem (Variables|Default|GetAttachableClass) _asbp_interact_actor_base) -1) (not (Variables|Default|GetLocked?)))))
    (:CastFailed
      (return false))))

(fn FindNewLockStatus
  (Variables|Default|SetLocked? true))