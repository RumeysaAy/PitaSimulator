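; Base actor for physics items the player can grab and release, driven by events from its BP_InteractableComponent.
; Grab asks the player controller via message calls whether an item is already held; if none is, it stops physics, hands itself over and disables collision on success.
; Release detaches the actor and restores collision and physics simulation.
; A text render shows physics and collision state every tick for debugging.
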(event OnPhysicsDisable(BP_InteractableComponent)
  (CallFunction|DisablePhysics))

(event OnGrab(BP_InteractableComponent)
  (CallFunction|Grab))

(event OnRelease(BP_InteractableComponent)
  (Transformation|DetachFromActor "KeepWorld" "KeepWorld" "KeepRelative")
  (Collision|SetActorEnableCollision true)
  (Physics|SetSimulatePhysics (Variables|Default|GetStaticMesh) true))

(event Custom|Grab
  (bind _grabbed (Class|BPIInteractionSystem|GetGrabbedItem(Message) (Game|GetPlayerController 0)))
  (if (not _grabbed)
    (Physics|SetSimulatePhysics (Variables|Default|GetStaticMesh) false)
    (bind _success (Class|BPIInteractionSystem|GrabItem(Message) (Game|GetPlayerController 0) (Variables|Default|GetBP_InteractableComponent) self))
    (if _success
      (CallFunction|DisablePhysics))))

(event Custom|DisablePhysics
  (Physics|SetSimulatePhysics (Variables|Default|GetStaticMesh) false)
  (Collision|SetActorEnableCollision false))

(event EventBeginPlay
  (|CallParentFunction) ; This node is disabled and will not be called.\nDrag off pins to build functionality.
)

(event Collision|EventActorBeginOverlap
  (params (OtherActor :type Actor%20Object%20Reference))
  (|CallParentFunction OtherActor) ; This node is disabled and will not be called.\nDrag off pins to build functionality.
)

(event EventTick
  (params (DeltaSeconds :type Float%20%28single-precision%29))
  (Rendering|Components|TextRender|SetText (Variables|Default|GetTextRender) (Utilities|Text|ToText(String) (Utilities|String|Append "Simulate Physics: " (Utilities|String|ToString(Boolean) (Physics|IsSimulatingPhysics (Variables|Default|GetStaticMesh) "None")) "
Collison Enabled: " (Utilities|String|ToString(Boolean) (Collision|GetActorEnableCollision))))))

(fn ConstructionScript
  (|CallParentFunction))