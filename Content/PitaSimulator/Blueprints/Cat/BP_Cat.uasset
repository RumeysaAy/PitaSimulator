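; Cat pawn for PitaSimulator that wanders to a target location and meows until the player deals with it.
; An enum state gates interaction, with timers and AI MoveTo driving movement and the looping meow.
; Interacting on arrival runs a delayed purr-text and sleep sequence before meowing resumes.
; Interacting in the idle state sends it to a hardcoded spot, then schedules its return after a random delay.
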(event OnInteractStart(BP_InteractableComponent)
  (if (Utilities|Enum|Equal(Enum) (Variables|Default|GetState) "NewEnumerator3")
    (Variables|Default|SetState "NewEnumerator0")
    (Utilities|Time|PauseTimerbyHandle (Variables|Default|GetMeowTimer))
    (Rendering|Components|TextRender|SetText (Variables|Default|GetTextRender) (Utilities|Text|MakeLiteralText "Mirr Mirr..."))
    (Utilities|FlowControl|Delay 5.0)
    (Variables|Default|SetState "NewEnumerator3")
    (Audio|Components|Audio|SetSound (Variables|Default|GetAudio) "/Game/PitaSimulator/Blueprints/Cat/Sound/cat-snarl_Cue.cat-snarl_Cue")
    (Audio|Components|Audio|Play (Variables|Default|GetAudio) 0.0)
    (Rendering|Components|TextRender|SetText (Variables|Default|GetTextRender) (Utilities|Text|MakeLiteralText "Zzzz..."))
    (Utilities|FlowControl|Delay 15.0)
    (Variables|Default|SetState "NewEnumerator0")
    (CallFunction|StartMeowing)
    (elif (Utilities|Enum|Equal(Enum) (Variables|Default|GetState) "NewEnumerator0")
      (Development|SetHiddeninGame (Variables|Default|GetTextRender) true false)
      (Variables|Default|SetState "NewEnumerator1")
      (Utilities|Time|PauseTimerbyHandle (Variables|Default|GetMeowTimer))
      (AI|AIMoveTo (Pawn|GetController) self "1765.000000,91.000000,0.000000" 0 5.0 false
        (:OnSuccess
          (Variables|Default|SetState "NewEnumerator0")
          (Utilities|Time|SetTimerbyEvent (delegate Custom|MoveToLocation) (Math|Random|RandomFloatinRange 5.0 1e+01)))))))

(event Custom|MoveToLocation
  (Variables|Default|SetState "NewEnumerator1")
  (AI|AIMoveTo (Pawn|GetController) self "0, 0, 0" (Variables|Default|GetCatLocation) 5.0 false
    (:OnSuccess
      (Variables|Default|SetState "NewEnumerator3")
      (CallFunction|StartMeowing))))

(event Custom|Meow
  (Audio|Components|Audio|Play (Variables|Default|GetAudio) 0.0))

(event Custom|StartMeowing
  (Rendering|Components|TextRender|SetText (Variables|Default|GetTextRender) (Utilities|Text|MakeLiteralText "Meow!"))
  (Development|SetHiddeninGame (Variables|Default|GetTextRender) false false)
  (Audio|Components|Audio|SetSound (Variables|Default|GetAudio) "/Game/PitaSimulator/Blueprints/Cat/Sound/cat-meow-Cue.cat-meow-Cue")
  (bind _returnvalue (Utilities|Time|SetTimerbyEvent (delegate Custom|Meow) 5.0 true))
  (Variables|Default|SetMeowTimer _returnvalue))

(event EventBeginPlay
  (Variables|Default|SetState "NewEnumerator0")
  (Utilities|Time|SetTimerbyEvent (delegate Custom|MoveToLocation) (Math|Random|RandomFloatinRange 3.0 5.0)))

(event Collision|EventActorBeginOverlap
  (params (OtherActor :type Actor%20Object%20Reference)))

(event EventTick
  (params (DeltaSeconds :type Float%20%28single-precision%29)))

(fn ConstructionScript)