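; Customer character in a pita shop game that queues along a spline, orders a plain or egg pita, and leaves once served.
; UpdateLocation AI-moves it to its queue slot; at the front it shows the serve sphere and announces a random order.
; ServeCustomer plays an angry or pay montage, fires served, money and pita events, then carries the pita out along the exit spline and self-destroys.
; Construction picks a VIP or random mesh.
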(event Custom|UpdateLocation
  (params (QueueOrder :type Integer) (bExit :type Boolean))
  (Variables|Default|SetQueueOrder QueueOrder)
  (if (not bExit)
    (AI|AIMoveTo (Pawn|GetController) self (.location (Spline|GetTransformatTime (Variables|Default|GetQueueSpline) (/ (Math|Conversions|ToFloat(Integer) (- (Variables|Default|GetQueueLimit) (Variables|Default|GetQueueOrder))) (Variables|Default|GetQueueLimit)) "World" false false)) 0 5.0 false
      (:OnSuccess
        (bind _output_get (Variables|Default|SetbCustomerReadyToServe (== (Variables|Default|GetQueueOrder) 0)))
        (if _output_get
          (CallFunction|MakeCustomerReady))))))

(event Custom|ServeCustomer
  (params (Burnt :type Boolean) (Egg :type Boolean))
  (if (Variables|Default|GetbCustomerReadyToServe)
    (Utilities|FlowControl|Sequence
      (:then_0
        (if Burnt
          (bind _returnvalue (Animation|PlayAnimMontage "/Game/PitaSimulator/Blueprints/Customer/Anim/Angry_Montage.Angry_Montage" 1.0 "None"))
          (Utilities|FlowControl|Delay _returnvalue)
          (else
            (bind _returnvalue_2 (Animation|PlayAnimMontage "/Game/PitaSimulator/Blueprints/Customer/Anim/Pay_Montage.Pay_Montage" 1.0 "None"))
            (Utilities|FlowControl|Delay _returnvalue_2)))
        (Default|CallOnServed)
        (Default|CallOnMoney (Variables|Default|GetisVIP))
        (Animation|PlayAnimMontage "/Game/PitaSimulator/Blueprints/Customer/Anim/Carrying_Montage.Carrying_Montage" 1.0 "None")
        (Default|CallOnPita)
        (Rendering|Material|SetMaterial (Variables|Default|GetPitaMesh) 0 (select Burnt "/InterchangeAssets/Materials/SheenMaterial_MR.SheenMaterial_MR" (select Egg "/Engine/EditorMaterials/Utilities/LinearColorPicker_MATInst.LinearColorPicker_MATInst" "/Engine/EngineDebugMaterials/ShadedLevelColorationLitMaterial.ShadedLevelColorationLitMaterial")))
        (Development|SetHiddeninGame (Variables|Default|GetPitaMesh) false false)
        (Development|SetHiddeninGame (Variables|Default|GetServeSphere) true true)
        (AI|AIMoveTo (Pawn|GetController) self (.location (Spline|GetTransformatSplinePoint (Variables|Default|GetExitSpline) 1 "World" false)) 0 5.0 false
          (:OnSuccess
            (AI|AIMoveTo (Pawn|GetController) self (.location (Spline|GetTransformatTime (Variables|Default|GetExitSpline) 1.0 "World" false false)) 0 5.0 false
              (:OnSuccess
                (Actor|DestroyActor)))))))))

(event Custom|MakeCustomerReady
  (Development|SetHiddeninGame (Variables|Default|GetServeSphere) false true)
  (bind _output_get (Variables|Default|SetEgg (> (Math|Random|RandomFloat) 0.75)))
  (Rendering|Components|TextRender|SetText (Variables|Default|GetTextRender) (select _output_get "Yumurtali Pide" "Pide"))
  (Default|CallOnCustomerReady (select _output_get "Yumurtali Pide" "Pide") (Variables|Default|GetEgg)))

(event EventBeginPlay
  (Development|SetHiddeninGame (Variables|Default|GetServeSphere) true true)
  (bind _returnvalue (Rendering|Material|CreateDynamicMaterialInstance (Variables|Default|GetPitaMesh) 0 "/AnimationSharing/AnimSharingRed.AnimSharingRed" "None" :!class /Script/Engine.PrimitiveComponent))
  (Rendering|Material|SetScalarParameterValue _returnvalue "BakeProgress" 1.0 :!class /Script/Engine.MaterialInstanceDynamic))

(event Collision|EventActorBeginOverlap
  (params (OtherActor :type Actor%20Object%20Reference)))

(fn ConstructionScript
  (Components|SkeletalMesh|SetSkeletalMeshAsset (Variables|Character|GetMesh) (select (Variables|Default|GetisVIP) "/Game/PitaSimulator/Blueprints/Customer/Art/Ch33/Ch33_nonPBR.Ch33_nonPBR" (.OutItem (Utilities|Array|Random (Utilities|Array|MakeArray "/Game/PitaSimulator/Blueprints/Customer/Art/Ch22/Ch22_nonPBR.Ch22_nonPBR" "/Game/PitaSimulator/Blueprints/Customer/Art/Ch31/Ch31_nonPBR.Ch31_nonPBR" "/Game/PitaSimulator/Blueprints/Customer/Art/Ch02/Ch02_nonPBR.Ch02_nonPBR" "/Game/PitaSimulator/Blueprints/Customer/Art/Ch04/Ch04_nonPBR.Ch04_nonPBR"))))))