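; BP_Queue is the customer line actor for the pita simulator, spawning customers along a spline and tracking who is next to serve.
; It spawns one customer at start, then another on a looping timer, pausing that timer once the queue is full.
; Each customer gets the queue and exit splines and a random VIP chance.
; Ready and served events are relayed outward, and serving removes the front customer and shifts the rest forward.
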(event Custom|CreateNewCustomer
  (bind _returnvalue (Game|SpawnActorfromClass "/Game/PitaSimulator/Blueprints/Customer/BP_Customer.BP_Customer_C" (Spline|GetTransformatTime (Variables|Default|GetQueueSpline) 0.0 "World" false false) "Undefined" "MultiplyWithRoot" 0 (Variables|Default|GetQueueSpline) (Variables|Default|GetQueueLimit) (Variables|Default|GetExitSpline) (> (Math|Random|RandomFloat) 0.8) 0))
  (Variables|Default|SetLastCreatedCustomer _returnvalue)
  (EventDispatchers|AssignOnServed (Variables|Default|GetLastCreatedCustomer) (delegate Custom|OnServed_Event))
  (EventDispatchers|BindEventtoOnCustomerReady (Variables|Default|GetLastCreatedCustomer) (delegate Custom|OnCustomerReady_Event))
  (bind _returnvalue_2 (Utilities|Array|Add (Variables|Default|GetQueue) (Variables|Default|GetLastCreatedCustomer)))
  (Default|UpdateLocation (Variables|Default|GetLastCreatedCustomer) _returnvalue_2 false))

(event Custom|UpdateQueueLocations
  (for (_array_element _array_index) (Variables|Default|GetQueue)
    (Default|UpdateLocation _array_element _array_index false)))

(event Custom|CreateAutoCustomers
  (if (< (Utilities|Array|Length (Variables|Default|GetQueue)) 7)
    (CallFunction|CreateNewCustomer)
    (else
      (Utilities|Time|PauseTimerbyHandle (Variables|Default|GetCreateAutoCustomersTimer)))))

(event Custom|OnServed_Event
  (Utilities|Array|RemoveIndex (Variables|Default|GetQueue))
  (CallFunction|UpdateQueueLocations)
  (Default|CallOnCustomerServed)
  (Variables|Default|SetIsThereAnyCustomerToServe false))

(event Custom|OnCustomerReady_Event
  (params (Pita :type Text) (Egg :type Boolean))
  (Default|CallOnCustomerReady Pita Egg)
  (Variables|Default|SetIsThereAnyCustomerToServe true))

(event EventBeginPlay
  (Utilities|FlowControl|Sequence
    (:then_1
      (CallFunction|CreateNewCustomer)
      (bind _returnvalue (Utilities|Time|SetTimerbyEvent (delegate Custom|CreateAutoCustomers) 3e+01 true))
      (Variables|Default|SetCreateAutoCustomersTimer _returnvalue))))

(event Collision|EventActorBeginOverlap
  (params (OtherActor :type Actor%20Object%20Reference)))

(event EventTick
  (params (DeltaSeconds :type Float%20%28single-precision%29)))

(fn ConstructionScript)

(fn ServeCustomer
  (params (Egg :type Boolean) (Burnt :type Boolean))
  (bind _queue (Variables|Default|GetQueue))
  (bind _output (Utilities|Array|Get(acopy) _queue))
  (Default|ServeCustomer _output Burnt Egg)
  (return _output))