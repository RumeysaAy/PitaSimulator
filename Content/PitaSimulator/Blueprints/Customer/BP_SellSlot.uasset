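; Sell counter slot where a pita is handed over to the waiting customer in exchange for money.
; It accepts only cooked or burnt pitas whose egg option matches the order reported by the customer Queue.
; Attaching one clears the slot and asks the Queue to serve, binding callbacks that destroy the pita and spawn BP_Money at arrow components.
; Payout is higher for VIPs and properly cooked pitas, with short delays staggering the spawns.
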(event Custom|OnCustomerReady_Event
  (params (Pita :type Text) (Egg :type Boolean))
  (Variables|Default|SetEgg Egg))

(event Custom|OnCustomerServed_Event)

(event Custom|OnMoney_Event
  (params (isVIP :type Boolean))
  (Variables|Default|SetisCooked (Utilities|Enum|Equal(Enum) (Variables|/Game/PitaSimulator/Blueprints/Pita/BP_Pita.BP_Pita_C|GetState (Variables|Default|GetAs%20BP%20Pita)) "NewEnumerator2"))
  (if isVIP
    (if (Variables|Default|GetisCooked)
      (Game|SpawnActorfromClass "/Game/PitaSimulator/Blueprints/Economy/BP_Money.BP_Money_C" (Transformation|GetWorldTransform (Variables|Default|GetArrow)) "Undefined" "MultiplyWithRoot" 0 10 0)
      (Utilities|FlowControl|Delay 0.2)
      (Game|SpawnActorfromClass "/Game/PitaSimulator/Blueprints/Economy/BP_Money.BP_Money_C" (Transformation|GetWorldTransform (Variables|Default|GetArrow1)) "Undefined" "MultiplyWithRoot" 0 10 0)
      (Game|SpawnActorfromClass "/Game/PitaSimulator/Blueprints/Economy/BP_Money.BP_Money_C" (Transformation|GetWorldTransform (Variables|Default|GetArrow)) "Undefined" "MultiplyWithRoot" 0 10 0)
      (Utilities|FlowControl|Delay 0.2)
      (Game|SpawnActorfromClass "/Game/PitaSimulator/Blueprints/Economy/BP_Money.BP_Money_C" (Transformation|GetWorldTransform (Variables|Default|GetArrow1)) "Undefined" "MultiplyWithRoot" 0 10 0)
      (else
        (Game|SpawnActorfromClass "/Game/PitaSimulator/Blueprints/Economy/BP_Money.BP_Money_C" (Transformation|GetWorldTransform (Variables|Default|GetArrow)) "Undefined" "MultiplyWithRoot" 0 10 0)
        (Utilities|FlowControl|Delay 0.2)
        (Game|SpawnActorfromClass "/Game/PitaSimulator/Blueprints/Economy/BP_Money.BP_Money_C" (Transformation|GetWorldTransform (Variables|Default|GetArrow1)) "Undefined" "MultiplyWithRoot" 0 10 0)))
    (elif (Variables|Default|GetisCooked)
      (Game|SpawnActorfromClass "/Game/PitaSimulator/Blueprints/Economy/BP_Money.BP_Money_C" (Transformation|GetWorldTransform (Variables|Default|GetArrow)) "Undefined" "MultiplyWithRoot" 0 10 0)
      (Utilities|FlowControl|Delay 0.2)
      (Game|SpawnActorfromClass "/Game/PitaSimulator/Blueprints/Economy/BP_Money.BP_Money_C" (Transformation|GetWorldTransform (Variables|Default|GetArrow1)) "Undefined" "MultiplyWithRoot" 0 10 0)
      (else
        (Game|SpawnActorfromClass "/Game/PitaSimulator/Blueprints/Economy/BP_Money.BP_Money_C" (Transformation|GetWorldTransform (Variables|Default|GetArrow)) "Undefined" "MultiplyWithRoot" 0 10 0)))))

(event Custom|OnPita_Event
  (Actor|DestroyActor (Variables|Default|GetAs%20BP%20Pita)))

(event EventBeginPlay
  (|CallParentFunction)
  (EventDispatchers|AssignOnCustomerReady (Variables|Default|GetQueue) (delegate Custom|OnCustomerReady_Event))
  (EventDispatchers|AssignOnCustomerServed (Variables|Default|GetQueue) (delegate Custom|OnCustomerServed_Event)))

(event Collision|EventActorBeginOverlap
  (params (OtherActor :type Actor%20Object%20Reference))
  (|CallParentFunction OtherActor) ; This node is disabled and will not be called.\nDrag off pins to build functionality.
)

(event EventTick
  (params (DeltaSeconds :type Float%20%28single-precision%29))
  (|CallParentFunction DeltaSeconds) ; This node is disabled and will not be called.\nDrag off pins to build functionality.
)

(event EventAttachFunction
  (params (AttachedActor :type Actor%20Object%20Reference))
  (bind _as_bp_pita (Variables|Default|GetAs%20BP%20Pita))
  (|CallParentFunction AttachedActor)
  (CallFunction|ClearSlot)
  (bind _currentcustomer (Default|ServeCustomer (Variables|Default|GetQueue) (Variables|/Game/PitaSimulator/Blueprints/Pita/BP_Pita.BP_Pita_C|GetEgg _as_bp_pita) (Utilities|Enum|Equal(Enum) (Variables|/Game/PitaSimulator/Blueprints/Pita/BP_Pita.BP_Pita_C|GetState _as_bp_pita) "NewEnumerator3")))
  (EventDispatchers|BindEventtoOnMoney _currentcustomer (delegate Custom|OnMoney_Event))
  (EventDispatchers|BindEventtoOnPita _currentcustomer (delegate Custom|OnPita_Event)))

(fn ConstructionScript
  (|CallParentFunction))

(fn CheckAttachable?
  (params (A :type Boolean) (Object :type Object%20Object%20Reference))
  (if (|CallParentFunction A Object)
    (if (Variables|/Game/PitaSimulator/Blueprints/Customer/BP_Queue.BP_Queue_C|GetIsThereAnyCustomerToServe (Variables|Default|GetQueue))
      (bind _asbp_pita (Utilities|Casting|CastToBP_Pita Object))
      (bind _output_get (Variables|Default|SetAs%20BP%20Pita _asbp_pita))
      (if (not (Class|KismetMathLibrary|XORBoolean (Variables|/Game/PitaSimulator/Blueprints/Pita/BP_Pita.BP_Pita_C|GetEgg _output_get) (Variables|Default|GetEgg)))
        (switch Utilities|FlowControl|Switch|SwitchonEPitaStates (Variables|/Game/PitaSimulator/Blueprints/Pita/BP_Pita.BP_Pita_C|GetState _asbp_pita)
          (:NewEnumerator0
            (return false))
          (:NewEnumerator1
            (return false))
          (:NewEnumerator2
            (return true))
          (:NewEnumerator3
            (return true)))
        (else
          (return false)))
      (else
        _)))
  (return false))