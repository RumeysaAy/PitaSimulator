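; BP_OrderPlace is an ordering station in the pita simulator where a button press buys a batch of ingredients.
; It binds to a child-actor BP_Button_Base's interaction event and, if the GameMode reports enough money, deducts a fixed price.
; It then spawns BP_Ingredient_Base actors at marker components for flour, water, two eggs and yeast.
; A Gate node blocks further orders for a ten-second cooldown after each purchase.
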(event Custom|OnButtonInteraction_Event
  (params (ButtonState :type EButtonState%20Enum :default "NewEnumerator0"))
  (Utilities|FlowControl|Gate false :!label _label
    (:Exit
      (bind _money (Class|BPIEconomy|GetCurrentMoney(Message) (Game|GetGameMode)))
      (if (>= _money 10)
        (Utilities|FlowControl|Sequence
          (:then_0
            (Class|BPIEconomy|RemoveMoney(Message) (Game|GetGameMode) 10))
          (:then_1
            (Game|SpawnActorfromClass "/Game/PitaSimulator/Blueprints/Ingredients/BP_Ingredient_Base.BP_Ingredient_Base_C" (Transformation|GetWorldTransform (Variables|Default|GetFlourLocation)) "Undefined" "MultiplyWithRoot" 0 "NewEnumerator0" 0)
            (Game|SpawnActorfromClass "/Game/PitaSimulator/Blueprints/Ingredients/BP_Ingredient_Base.BP_Ingredient_Base_C" (Transformation|GetWorldTransform (Variables|Default|GetWaterLocation)) "Undefined" "MultiplyWithRoot" 0 "NewEnumerator1" 0)
            (Game|SpawnActorfromClass "/Game/PitaSimulator/Blueprints/Ingredients/BP_Ingredient_Base.BP_Ingredient_Base_C" (Transformation|GetWorldTransform (Variables|Default|GetEgg1Location)) "Undefined" "MultiplyWithRoot" 0 "NewEnumerator2" 0)
            (Game|SpawnActorfromClass "/Game/PitaSimulator/Blueprints/Ingredients/BP_Ingredient_Base.BP_Ingredient_Base_C" (Transformation|GetWorldTransform (Variables|Default|GetEgg2Location)) "Undefined" "MultiplyWithRoot" 0 "NewEnumerator2" 0)
            (Game|SpawnActorfromClass "/Game/PitaSimulator/Blueprints/Ingredients/BP_Ingredient_Base.BP_Ingredient_Base_C" (Transformation|GetWorldTransform (Variables|Default|GetYeastLocation)) "Undefined" "MultiplyWithRoot" 0 "NewEnumerator3" 0))
          (:then_2
            (goto _label Close))
          (:then_3
            (Utilities|FlowControl|Delay 1e+01)
            (goto _label Open)))
        (else
          (goto _label Open))))))

(event EventBeginPlay
  (bind _asbp_button_base (Utilities|Casting|CastToBP_Button_Base (Variables|/Script/Engine.ChildActorComponent|GetChildActor (Variables|Default|GetButton))))
  (bind _output_get (Variables|Default|SetOrderButton _asbp_button_base))
  (EventDispatchers|AssignOnButtonInteraction _output_get (delegate Custom|OnButtonInteraction_Event)))

(event Collision|EventActorBeginOverlap
  (params (OtherActor :type Actor%20Object%20Reference)))

(event EventTick
  (params (DeltaSeconds :type Float%20%28single-precision%29)))

(fn ConstructionScript)