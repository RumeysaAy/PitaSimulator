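; BP_Package is an ingredient package actor that holds stock for flour, water, yeast and egg.
; On BeginPlay it casts the child actor in each of its four package slots to BP_Package_Stock and caches the references.
; AddIngredientsToPackage saves the incoming MarketList map, then passes each entry's value to the matching stock's ChangeStock, chosen by ingredient key.
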(event Custom|AddIngredientsToPackage
  (params (MarketList :type Map%20of%20EIngredients%20Enums%20to%20Integers :default "NewEnumerator0"))
  (bind _output_get (Variables|Default|SetMarketList MarketList))
  (bind _keys (Utilities|Map|Keys _output_get))
  (for _array_element _keys
    (Default|ChangeStock (Utilities|Select :Index _array_element :NewEnumerator0 (Variables|Default|GetFlourStock) :NewEnumerator1 (Variables|Default|GetWaterStock) :NewEnumerator2 (Variables|Default|GetEggStock) :NewEnumerator3 (Variables|Default|GetYeastStock)) (.Value (Utilities|Map|Find (Variables|Default|GetMarketList) _array_element)))))

(event EventBeginPlay
  (|CallParentFunction)
  (Utilities|FlowControl|Sequence
    (:then_0
      (bind _asbp_package_stock (Utilities|Casting|CastToBP_Package_Stock (Variables|/Script/Engine.ChildActorComponent|GetChildActor (Variables|Default|GetPackage_Slot_Flour))))
      (Variables|Default|SetFlourStock _asbp_package_stock))
    (:then_1
      (bind _asbp_package_stock_2 (Utilities|Casting|CastToBP_Package_Stock (Variables|/Script/Engine.ChildActorComponent|GetChildActor (Variables|Default|GetPackage_Slot_Water))))
      (Variables|Default|SetWaterStock _asbp_package_stock_2))
    (:then_2
      (bind _asbp_package_stock_3 (Utilities|Casting|CastToBP_Package_Stock (Variables|/Script/Engine.ChildActorComponent|GetChildActor (Variables|Default|GetPackage_Slot_Yeast))))
      (Variables|Default|SetYeastStock _asbp_package_stock_3))
    (:then_3
      (bind _asbp_package_stock_4 (Utilities|Casting|CastToBP_Package_Stock (Variables|/Script/Engine.ChildActorComponent|GetChildActor (Variables|Default|GetPackage_Slot_Egg))))
      (Variables|Default|SetEggStock _asbp_package_stock_4))))

(event Collision|EventActorBeginOverlap
  (params (OtherActor :type Actor%20Object%20Reference))
  (|CallParentFunction OtherActor) ; This node is disabled and will not be called.\nDrag off pins to build functionality.
)

(event EventTick
  (params (DeltaSeconds :type Float%20%28single-precision%29))
  (|CallParentFunction DeltaSeconds) ; This node is disabled and will not be called.\nDrag off pins to build functionality.
)

(fn ConstructionScript
  (|CallParentFunction))