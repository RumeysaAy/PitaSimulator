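; BP_PurchaseButton is a button for buying one ingredient type: flour, water, egg or yeast.
; Construction labels it with the ingredient name and creates a dynamic material showing that ingredient's idle texture.
; On button interaction it swaps to the selected texture and broadcasts OnIngredientPurchased with the type, regardless of button state.
; ResetButton restores the idle texture, while DisableButton is an empty stub.
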(event Custom|OnButtonInteraction_Event
  (params (ButtonState :type EButtonState%20Enum :default "NewEnumerator0"))
  (Rendering|Material|SetTextureParameterValue (Variables|Default|GetPurchaseButtonMat) "Color" (Utilities|Select :Index (Variables|Default|GetIngredientType) :NewEnumerator0 "/Game/PitaSimulator/Blueprints/Tablet/Icons/Flour_Selected.Flour_Selected" :NewEnumerator1 "/Game/PitaSimulator/Blueprints/Tablet/Icons/Water_Selected.Water_Selected" :NewEnumerator2 "/Game/PitaSimulator/Blueprints/Tablet/Icons/Egg_Selected.Egg_Selected" :NewEnumerator3 "/Game/PitaSimulator/Blueprints/Tablet/Icons/Yeast_Selected.Yeast_Selected"))
  (Default|CallOnIngredientPurchased (Variables|Default|GetIngredientType)))

(event Custom|DisableButton)

(event Custom|ResetButton
  (Rendering|Material|SetTextureParameterValue (Variables|Default|GetPurchaseButtonMat) "Color" (Utilities|Select :Index (Variables|Default|GetIngredientType) :NewEnumerator0 "/Game/PitaSimulator/Blueprints/Tablet/Icons/Flour_Idle.Flour_Idle" :NewEnumerator1 "/Game/PitaSimulator/Blueprints/Tablet/Icons/Water_Idle.Water_Idle" :NewEnumerator2 "/Game/PitaSimulator/Blueprints/Tablet/Icons/Egg_Idle.Egg_Idle" :NewEnumerator3 "/Game/PitaSimulator/Blueprints/Tablet/Icons/Yeast_Idle.Yeast_Idle")))

(event EventBeginPlay
  (|CallParentFunction)
  (EventDispatchers|AssignOnButtonInteraction (delegate Custom|OnButtonInteraction_Event)))

(event Collision|EventActorBeginOverlap
  (params (OtherActor :type Actor%20Object%20Reference))
  (|CallParentFunction OtherActor) ; This node is disabled and will not be called.\nDrag off pins to build functionality.
)

(event EventTick
  (params (DeltaSeconds :type Float%20%28single-precision%29))
  (|CallParentFunction DeltaSeconds) ; This node is disabled and will not be called.\nDrag off pins to build functionality.
)

(fn ConstructionScript
  (|CallParentFunction)
  (Rendering|Components|TextRender|SetText (Variables|Default|GetTextRender) (Utilities|Text|ToText(String) (Utilities|String|EnumtoString (Variables|Default|GetIngredientType))))
  (bind _returnvalue (Rendering|Material|CreateDynamicMaterialInstance (Variables|Default|GetStaticMesh) 0 "/Game/PitaSimulator/Blueprints/Tablet/Icons/M_PurchaseButton.M_PurchaseButton" "None" :!class /Script/Engine.PrimitiveComponent))
  (bind _output_get (Variables|Default|SetPurchaseButtonMat _returnvalue))
  (Rendering|Material|SetTextureParameterValue _output_get "Color" (Utilities|Select :Index (Variables|Default|GetIngredientType) :NewEnumerator0 "/Game/PitaSimulator/Blueprints/Tablet/Icons/Flour_Idle.Flour_Idle" :NewEnumerator1 "/Game/PitaSimulator/Blueprints/Tablet/Icons/Water_Idle.Water_Idle" :NewEnumerator2 "/Game/PitaSimulator/Blueprints/Tablet/Icons/Egg_Idle.Egg_Idle" :NewEnumerator3 "/Game/PitaSimulator/Blueprints/Tablet/Icons/Yeast_Idle.Yeast_Idle")))