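; BP_Package_Stock is an ingredient stock package that hands the player one ingredient per interaction and shows the remaining count.
; On interact, if the player controller holds nothing and stock remains, it spawns an ingredient of its type, passes it to the controller to grab, and decrements the count.
; ChangeStock updates the count and its text display, with an empty branch at zero.
; The construction script picks the mesh from the ingredient type.
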(event OnInteractStart(BP_InteractableComponent)
  (bind _grabbed (Class|BPIInteractionSystem|GetGrabbedItem(Message) (Game|GetPlayerController 0)))
  (if (not _grabbed)
    (if (> (Variables|Default|GetCount) 0)
      (bind _returnvalue (Game|SpawnActorfromClass (Variables|Default|GetIngredient) (Math|Transform|MakeTransform "0, 0, 0" "0, 0, 0" "1.000000,1.000000,1.000000") "Undefined" "MultiplyWithRoot" 0 (Variables|Default|GetIngredientType) 0))
      (Class|BPIInteractionSystem|GrabItem(Message) (Game|GetPlayerController 0) (Variables|/Game/PitaSimulator/InteractionSystem/BP_InteractActor_Base.BP_InteractActor_Base_C|GetBP_InteractableComponent _returnvalue) _returnvalue)
      (CallFunction|ChangeStock -1))))

(event Custom|ChangeStock
  (params (Value :type Integer))
  (Variables|Default|SetCount (+ (Variables|Default|GetCount) Value))
  (Rendering|Components|TextRender|SetText (Variables|Default|GetTextRender) (Utilities|Text|ToText(Integer) (Variables|Default|GetCount)))
  (if (== (Variables|Default|GetCount) 0)
    _))

(event EventBeginPlay
  (|CallParentFunction)
  (Rendering|Components|TextRender|SetText (Variables|Default|GetTextRender) (Utilities|Text|ToText(Integer) (Variables|Default|GetCount))))

(event Collision|EventActorBeginOverlap
  (params (OtherActor :type Actor%20Object%20Reference))
  (|CallParentFunction OtherActor) ; This node is disabled and will not be called.\nDrag off pins to build functionality.
)

(event EventTick
  (params (DeltaSeconds :type Float%20%28single-precision%29))
  (|CallParentFunction DeltaSeconds) ; This node is disabled and will not be called.\nDrag off pins to build functionality.
)

(fn ConstructionScript
  (|CallParentFunction)
  (Components|StaticMesh|SetStaticMesh (Variables|Default|GetStaticMesh) (Utilities|Select :Index (Variables|Default|GetIngredientType) :NewEnumerator0 "/Game/Fab/Flour_bag/sm_flourbag.sm_flourbag" :NewEnumerator1 "/Game/Fab/Water_Bottle_Free/Bottle_Water_perfect.Bottle_Water_perfect" :NewEnumerator2 "/Game/Fab/Soybean/soybean.soybean" :NewEnumerator3 "/Game/Fab/Yogurt/yeast_maya.yeast_maya")))