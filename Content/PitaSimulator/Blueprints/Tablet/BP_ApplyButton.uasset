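; BP_ApplyButton is a tablet Apply button that shows success or failure feedback.
; On BeginPlay it creates a dynamic instance of M_PurchaseButton on its static mesh and sets the idle texture.
; ShowResult swaps the Color texture parameter to the selected or not-applied texture based on Success, then restores idle after a one-second delay.
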(event Custom|ShowResult
  (params (Success :type Boolean))
  (Rendering|Material|SetTextureParameterValue (Variables|Default|GetApplyMaterial) "Color" (select Success "/Game/PitaSimulator/Blueprints/Tablet/Icons/Apply_Selected.Apply_Selected" "/Game/PitaSimulator/Blueprints/Tablet/Icons/Apply_Not.Apply_Not"))
  (Utilities|FlowControl|Delay 1.0)
  (Rendering|Material|SetTextureParameterValue (Variables|Default|GetApplyMaterial) "Color" "/Game/PitaSimulator/Blueprints/Tablet/Icons/Apply_Idle.Apply_Idle"))

(event EventBeginPlay
  (|CallParentFunction)
  (bind _returnvalue (Rendering|Material|CreateDynamicMaterialInstance (Variables|Default|GetStaticMesh) 0 "/Game/PitaSimulator/Blueprints/Tablet/Icons/M_PurchaseButton.M_PurchaseButton" "None" :!class /Script/Engine.PrimitiveComponent))
  (bind _output_get (Variables|Default|SetApplyMaterial _returnvalue))
  (Rendering|Material|SetTextureParameterValue _output_get "Color" "/Game/PitaSimulator/Blueprints/Tablet/Icons/Apply_Idle.Apply_Idle"))

(event Collision|EventActorBeginOverlap
  (params (OtherActor :type Actor%20Object%20Reference))
  (|CallParentFunction OtherActor) ; This node is disabled and will not be called.\nDrag off pins to build functionality.
)

(event EventTick
  (params (DeltaSeconds :type Float%20%28single-precision%29))
  (|CallParentFunction DeltaSeconds) ; This node is disabled and will not be called.\nDrag off pins to build functionality.
)

(fn ConstructionScript
  (|CallParentFunction))