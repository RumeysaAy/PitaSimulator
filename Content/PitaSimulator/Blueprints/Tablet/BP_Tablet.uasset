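; BP_Tablet is an in-game shop tablet for ordering ingredients.
; Child-actor purchase buttons broadcast ingredient types, which it tallies in a map at a flat unit price and lists with the total on a text render.
; The apply button checks and deducts money through game mode messages, then sends the order to the BP_Package found in the level.
; Successful or unaffordable orders reset the list and buttons, and the apply button shows the result.
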(event Custom|ResetList
  (Variables|Default|SetTotalPrice 0)
  (Utilities|Map|Clear (Variables|Default|GetMarketList))
  (Rendering|Components|TextRender|SetText (Variables|Default|GetTextRender) (Utilities|Text|MakeLiteralText " "))
  (for _array_element (Components|GetChildrenComponents (Variables|Default|GetBackground) false)
    (bind _aschild_actor_component (Utilities|Casting|CastToChildActorComponent _array_element))
    (bind _asbp_purchase_button (Utilities|Casting|CastToBP_PurchaseButton (Variables|/Script/Engine.ChildActorComponent|GetChildActor _aschild_actor_component)))
    (Default|ResetButton _asbp_purchase_button)))

(event Custom|OnIngredientPurchased_Event
  (params (IngredientType :type EIngredients%20Enum :default "NewEnumerator0"))
  (bind _marketlist (Variables|Default|GetMarketList))
  (bind (_value _returnvalue) (Utilities|Map|Find _marketlist IngredientType))
  (Development|PrintString (Utilities|String|EnumtoString IngredientType))
  (Variables|Default|SetTotalPrice (+ (Variables|Default|GetTotalPrice) 2))
  (if _returnvalue
    (Utilities|Map|Add _marketlist IngredientType (+ _value 1))
    (else
      (Utilities|Map|Add _marketlist IngredientType 1)))
  (bind _keys (Utilities|Map|Keys (Variables|Default|GetMarketList)))
  (Variables|Default|SetMarketListString "")
  (for _array_element _keys
    (Variables|Default|SetMarketListString (Utilities|String|Append (Variables|Default|GetMarketListString) (Utilities|String|EnumtoString _array_element) " " (Utilities|String|ToString(Integer) (.Value (Utilities|Map|Find (Variables|Default|GetMarketList) _array_element))) "
")))
  (Rendering|Components|TextRender|SetText (Variables|Default|GetTextRender) (Utilities|Text|ToText(String) (Utilities|String|Append (Variables|Default|GetMarketListString) "Total Price: " (Utilities|String|ToString(Integer) (Variables|Default|GetTotalPrice))))))

(event Custom|OnButtonInteraction_Event
  (params (ButtonState :type EButtonState%20Enum :default "NewEnumerator0"))
  (if (Utilities|Map|IsEmpty (Variables|Default|GetMarketList))
    (Default|ShowResult (Variables|Default|GetAs%20BP%20Apply%20Button) false)
    (else
      (bind _money (Class|BPIEconomy|GetCurrentMoney(Message) (Game|GetGameMode)))
      (if (>= _money (Variables|Default|GetTotalPrice))
        (Class|BPIEconomy|RemoveMoney(Message) (Game|GetGameMode) (Variables|Default|GetTotalPrice))
        (bind _returnvalue (Actor|GetActorOfClass "/Game/PitaSimulator/Blueprints/Tablet/BP_Package.BP_Package_C"))
        (Default|AddIngredientstoPackage _returnvalue (Variables|Default|GetMarketList))
        (CallFunction|ResetList)
        (Default|ShowResult (Variables|Default|GetAs%20BP%20Apply%20Button) true)
        (else
          (CallFunction|ResetList)
          (Default|ShowResult (Variables|Default|GetAs%20BP%20Apply%20Button) false))))))

(event EventBeginPlay
  (Utilities|FlowControl|Sequence
    (:then_0
      (for _array_element (Components|GetChildrenComponents (Variables|Default|GetBackground) false)
        (bind _aschild_actor_component (Utilities|Casting|CastToChildActorComponent _array_element))
        (bind _asbp_purchase_button (Utilities|Casting|CastToBP_PurchaseButton (Variables|/Script/Engine.ChildActorComponent|GetChildActor _aschild_actor_component)))
        (EventDispatchers|AssignOnIngredientPurchased _asbp_purchase_button (delegate Custom|OnIngredientPurchased_Event))))
    (:then_1
      (bind _asbp_apply_button (Utilities|Casting|CastToBP_ApplyButton (Variables|/Script/Engine.ChildActorComponent|GetChildActor (Variables|Default|GetApplyButton))))
      (bind _output_get (Variables|Default|SetAs%20BP%20Apply%20Button _asbp_apply_button))
      (EventDispatchers|AssignOnButtonInteraction _output_get (delegate Custom|OnButtonInteraction_Event)))))

(event Collision|EventActorBeginOverlap
  (params (OtherActor :type Actor%20Object%20Reference)))

(event EventTick
  (params (DeltaSeconds :type Float%20%28single-precision%29)))

(fn ConstructionScript)