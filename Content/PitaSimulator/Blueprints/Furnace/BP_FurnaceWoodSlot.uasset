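; Furnace wood slot, a child of an attachable-slot Blueprint, that holds up to three pieces of wood as fuel.
; Each added piece snaps to the location matching the count and restarts the burn timer.
; When the timer fires, it destroys the last piece in the list and restarts while wood remains.
; Dispatchers signal when the first piece starts the burn and when the slot empties.
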(event EventBeginPlay
  (|CallParentFunction) ; This node is disabled and will not be called.\nDrag off pins to build functionality.
)

(event Collision|EventActorBeginOverlap
  (params (OtherActor :type Actor%20Object%20Reference))
  (|CallParentFunction OtherActor) ; This node is disabled and will not be called.\nDrag off pins to build functionality.
)

(event EventTick
  (params (DeltaSeconds :type Float%20%28single-precision%29))
  (|CallParentFunction DeltaSeconds) ; This node is disabled and will not be called.\nDrag off pins to build functionality.
)

(fn ConstructionScript
  (|CallParentFunction))

(fn CheckAttachable?
  (params (A :type Boolean) (Object :type Object%20Object%20Reference))
  (if (|CallParentFunction A Object)
    (return (< (Utilities|Array|Length (Variables|Default|GetAttachedActors)) 3))
    (else
      (return false))))

(fn FindNewLockStatus
  (Transformation|AttachComponentToComponent (Variables|Default|GetGrabbed%20Actor) (Utilities|Select :Index (Utilities|Array|Length (Variables|Default|GetAttachedActors)) :Option%200 0 :Option%201 (Variables|Default|GetWood1Location) :Option%202 (Variables|Default|GetWood2Location) :Option%203 (Variables|Default|GetWood3Location)) "None" "SnapToTarget" "SnapToTarget" "KeepRelative" true)
  (bind _returnvalue (Utilities|Time|SetTimerbyFunctionName 0 "BurnWood" (Variables|Default|GetBurnTime)))
  (Variables|Default|SetBurnTimer _returnvalue)
  (if (== (Utilities|Array|Length (Variables|Default|GetAttachedActors)) 1)
    (Default|CallOnFurnaceWoodSlotActive)
    (Variables|Default|SetIsBurning true)))

(fn BurnWood
  (bind _attachedactors (Variables|Default|GetAttachedActors))
  (bind _output_get (LocalVariables|SetRemovedWood (Utilities|Array|Get(acopy) _attachedactors (Utilities|Array|LastIndex _attachedactors))))
  (Utilities|Array|RemoveItem (Variables|Default|GetAttachedActors) _output_get)
  (Actor|DestroyActor _output_get)
  (if (Utilities|Array|IsEmpty (Variables|Default|GetAttachedActors))
    (Variables|Default|SetIsBurning false)
    (Default|CallOnFurnaceWoodSlotEmpty)
    (else
      (bind _returnvalue (Utilities|Time|SetTimerbyFunctionName 0 "BurnWood" (Variables|Default|GetBurnTime)))
      (Variables|Default|SetBurnTimer _returnvalue))))