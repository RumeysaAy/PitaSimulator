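; Furnace manager actor that links two wood slots to two furnace slots and tracks whether the furnace is burning.
; It binds to the wood slots' events: either becoming active sets both furnace slots burning.
; When one empties, the furnace slots stop only if neither wood slot is still burning.
; Tick updates a text render with the current burning state.
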(event Custom|OnFurnaceWoodSlotActive_Event
  (Variables|Default|SetbBurning true)
  (Default|SetFurnaceBurning (Variables|Default|GetFurnaceSlot1) (Variables|Default|GetbBurning)))

(event Custom|OnFurnaceWoodSlotEmpty_Event
  (bind _output_get (Variables|Default|SetbBurning (or (Variables|/Game/PitaSimulator/Blueprints/Furnace/BP_FurnaceWoodSlot.BP_FurnaceWoodSlot_C|GetIsBurning (Variables|Default|GetFurnaceWoodSlot1)) (Variables|/Game/PitaSimulator/Blueprints/Furnace/BP_FurnaceWoodSlot.BP_FurnaceWoodSlot_C|GetIsBurning (Variables|Default|GetFurnaceWoodSlot2)))))
  (if (not _output_get)
    (Default|SetFurnaceBurning (Variables|Default|GetFurnaceSlot1) false)))

(event EventBeginPlay
  (bind _furnacewoodslot1 (Variables|Default|GetFurnaceWoodSlot1))
  (EventDispatchers|AssignOnFurnaceWoodSlotActive _furnacewoodslot1 (delegate Custom|OnFurnaceWoodSlotActive_Event))
  (EventDispatchers|BindEventtoOnFurnaceWoodSlotEmpty _furnacewoodslot1 (delegate Custom|OnFurnaceWoodSlotEmpty_Event)))

(event Collision|EventActorBeginOverlap
  (params (OtherActor :type Actor%20Object%20Reference)))

(event EventTick
  (params (DeltaSeconds :type Float%20%28single-precision%29))
  (Rendering|Components|TextRender|SetText (Variables|Default|GetTextRender) (select (Variables|Default|GetbBurning) (Utilities|Text|MakeLiteralText "Burning") (Utilities|Text|MakeLiteralText "Not burning"))))

(fn ConstructionScript)