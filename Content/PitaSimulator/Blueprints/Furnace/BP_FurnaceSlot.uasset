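; BP_FurnaceSlot is an interactable furnace slot that swaps a pita with the slot on the player's held peel and controls its cooking.
; On interaction it casts the grabbed actor to BP_Peel and reaches that peel's BP_PitaSlot child actor.
; A locked slot hands its pita to an empty peel and stops cooking.
; An unlocked slot takes the peel's pita through AttachFunction and starts cooking, with Turkish debug prints reporting the state.
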(event OnInteractStart(BP_InteractableComponent)
  (bind _attachedactors (Variables|Default|GetAttachedActors))
  (bind _output (Utilities|Array|Get(acopy) _attachedactors))
  (bind _grabbedactor (Class|BPIInteractionSystem|GetGrabbedItem(Message) (Game|GetPlayerController 0)))
  (bind _asbp_peel (Utilities|Casting|CastToBP_Peel _grabbedactor))
  (Variables|Default|SetAs%20BP%20Peel _asbp_peel)
  (if (Variables|Default|GetLocked?)
    (Development|PrintString "Zaten pide var!")
    (bind _asbp_pita_slot (Utilities|Casting|CastToBP_PitaSlot (Variables|/Script/Engine.ChildActorComponent|GetChildActor (Variables|/Game/PitaSimulator/Blueprints/Peel/BP_Peel.BP_Peel_C|GetPitaSlot2 (Variables|Default|GetAs%20BP%20Peel)))))
    (if (== (Utilities|Array|Length (Variables|/Game/PitaSimulator/InteractionSystem/ItemSlot/BP_ItemSlot_Base.BP_ItemSlot_Base_C|GetAttachedActors _asbp_pita_slot)) 0)
      (Default|AttachFunction _asbp_pita_slot _output)
      (bind _asbp_pita (Utilities|Casting|CastToBP_Pita _output))
      (Default|StopCooking _asbp_pita)
      (Utilities|Array|Clear (Variables|Default|GetAttachedActors))
      (Variables|Default|SetLocked? false))
    (else
      (bind _asbp_pita_slot_2 (Utilities|Casting|CastToBP_PitaSlot (Variables|/Script/Engine.ChildActorComponent|GetChildActor (Variables|/Game/PitaSimulator/Blueprints/Peel/BP_Peel.BP_Peel_C|GetPitaSlot2 (Variables|Default|GetAs%20BP%20Peel)))))
      (if (== (Utilities|Array|Length (Variables|/Game/PitaSimulator/InteractionSystem/ItemSlot/BP_ItemSlot_Base.BP_ItemSlot_Base_C|GetAttachedActors _asbp_pita_slot_2)) 1)
        (CallFunction|AttachFunction (Utilities|Array|Get(acopy) (Variables|/Game/PitaSimulator/InteractionSystem/ItemSlot/BP_ItemSlot_Base.BP_ItemSlot_Base_C|GetAttachedActors _asbp_pita_slot_2)))
        (Utilities|Array|Clear (Variables|/Game/PitaSimulator/InteractionSystem/ItemSlot/BP_ItemSlot_Base.BP_ItemSlot_Base_C|GetAttachedActors _asbp_pita_slot_2))
        (Variables|/Game/PitaSimulator/InteractionSystem/ItemSlot/BP_ItemSlot_Base.BP_ItemSlot_Base_C|SetLocked? _asbp_pita_slot_2 false)
        (Development|PrintString "Pide var! neye baktın?")
        (bind _asbp_pita_2 (Utilities|Casting|CastToBP_Pita (Utilities|Array|Get(acopy) (Variables|Default|GetAttachedActors))))
        (Default|StartCooking _asbp_pita_2)
        (else
          (Development|PrintString "Pide yok."))))))

(event EventBeginPlay
  (|CallParentFunction) ; This node is disabled and will not be called.\nDrag off pins to build functionality.
)

(event Collision|EventActorBeginOverlap
  (params (OtherActor :type Actor%20Object%20Reference))
  (|CallParentFunction OtherActor) ; This node is disabled and will not be called.\nDrag off pins to build functionality.
)

(event EventTick
  (params (DeltaSeconds :type Float%20%28single-precision%29))
  (|CallParentFunction DeltaSeconds) ; This node is disabled and will not be called.\nDrag off pins to build functionality.
)

(fn ConstructionScript
  (|CallParentFunction))