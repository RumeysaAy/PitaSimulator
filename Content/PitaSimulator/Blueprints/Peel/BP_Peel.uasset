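; BP_Peel is a grabbable peel actor in PitaSimulator that carries a pita slot as a child actor.
; It responds to the grab and release events of its BP_InteractableComponent.
; Grabbing disables collision on the PitaSlot2 child actor, and releasing enables it again.
; BeginPlay, overlap, Tick and the construction script add no logic of their own.
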(event OnGrab(BP_InteractableComponent)
  (Collision|SetActorEnableCollision (Variables|/Script/Engine.ChildActorComponent|GetChildActor (Variables|Default|GetPitaSlot2)) false))

(event OnRelease(BP_InteractableComponent)
  (Collision|SetActorEnableCollision (Variables|/Script/Engine.ChildActorComponent|GetChildActor (Variables|Default|GetPitaSlot2)) true))

(event EventBeginPlay
  (|CallParentFunction) ; This node is disabled and will not be called.\nDrag off pins to build functionality.
)

(event Collision|EventActorBeginOverlap
  (params (OtherActor :type Actor%20Object%20Reference))
  (|CallParentFunction OtherActor) ; This node is disabled and will not be called.\nDrag off pins to build functionality.
)

(event EventTick
  (params (DeltaSeconds :type Float%20%28single-precision%29))
  (|CallParentFunction DeltaSeconds) ; This node is disabled and will not be called.\nDrag off pins to build functionality.
)

(fn ConstructionScript
  (|CallParentFunction))