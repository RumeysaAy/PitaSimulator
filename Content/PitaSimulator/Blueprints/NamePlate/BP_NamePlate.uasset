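; BP_NamePlate is an interactable nameplate actor that shows the bakery's name and opens a naming UI in the Pita Simulator game.
; It binds to the game mode's bakery name changed event and updates its NameText to match.
; Interacting through BP_InteractableComponent switches the first player to UI-only input with a visible cursor and adds a WBP_NamePlate widget to the viewport.
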(event OnInteractStart(BP_InteractableComponent)
  (bind _returnvalue (Game|GetPlayerController 0))
  (Input|SetInputModeUIOnly _returnvalue 0 "DoNotLock" false)
  (Variables|/Script/Engine.PlayerController|SetbShowMouseCursor _returnvalue true)
  (bind _returnvalue_2 (UserInterface|CreateWidget "/Game/PitaSimulator/Blueprints/NamePlate/WBP_NamePlate.WBP_NamePlate_C"))
  (UserInterface|Viewport|AddtoViewport _returnvalue_2 0))

(event Custom|OnBakeryNameChanged_Event
  (params (NewBakeryName :type Name))
  (Rendering|Components|TextRender|SetText (Variables|Default|GetNameText) (Utilities|Text|ToText(Name) NewBakeryName)))

(event EventBeginPlay
  (bind _asbp_pita_game_mode (Utilities|Casting|CastToBP_PitaGameMode (Game|GetGameMode)))
  (EventDispatchers|BindEventtoOnBakeryNameChanged _asbp_pita_game_mode (delegate Custom|OnBakeryNameChanged_Event)))

(event Collision|EventActorBeginOverlap
  (params (OtherActor :type Actor%20Object%20Reference)))

(event EventTick
  (params (DeltaSeconds :type Float%20%28single-precision%29)))

(fn ConstructionScript)