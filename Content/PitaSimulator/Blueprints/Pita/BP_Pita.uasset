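; BP_Pita is a grabbable pita that cooks over time in a pita-making simulator.
; StartCooking plays CookTimeline, which tints a dynamic material and advances State from cooking to cooked to burnt, revealing smoke once cooked; StopCooking halts it.
; Interacting with a held BP_EggBrush sets Egg and yellows the dough, while grabbing unlocks its DoughStand slot.
; Tick displays the current state on a TextRender.
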(event OnGrab(BP_InteractableComponent)
  (Default|UnlockSlot (Variables|Default|GetDoughStand)))

(event OnInteractStart(BP_InteractableComponent)
  (bind (_grabbed _grabbedactor) (Class|BPIInteractionSystem|GetGrabbedItem(Message) (Game|GetPlayerController 0)))
  (if _grabbed
    (Utilities|Casting|CastToBP_EggBrush _grabbedactor)
    (Variables|Default|SetEgg true)
    (Rendering|Material|SetVectorParameterValue (Variables|Default|GetPitaMaterialInstance) "Color" "(R=1.000000,G=0.966577,B=0.000000,A=1.000000)" :!class /Script/Engine.MaterialInstanceDynamic)))

(event Custom|StartCooking
  (Development|PrintString "Pide pişmeye başladı.")
  (Variables|Default|SetState "NewEnumerator1")
  (bind _color (Timeline|CookTimeline Play)
    (:Update
      (Rendering|Material|SetVectorParameterValue (Variables|Default|GetPitaMaterialInstance) "Color" _color :!class /Script/Engine.MaterialInstanceDynamic))
    (:CookStateChange
      (bind _output_get (Variables|Default|SetState (Utilities|Select :Index (Variables|Default|GetState) :NewEnumerator0 "NewEnumerator1" :NewEnumerator1 "NewEnumerator2" :NewEnumerator2 "NewEnumerator3" :NewEnumerator3 "NewEnumerator3")))
      (if (Utilities|Enum|Equal(Enum) _output_get "NewEnumerator2")
        (Development|SetHiddeninGame (Variables|Default|GetSmokes) false true)))))

(event Custom|StopCooking
  (Development|PrintString "Pide artık pişmiyor.")
  (bind _color (Timeline|CookTimeline Stop)
    (:Update
      (Rendering|Material|SetVectorParameterValue (Variables|Default|GetPitaMaterialInstance) "Color" _color :!class /Script/Engine.MaterialInstanceDynamic))
    (:CookStateChange
      (bind _output_get (Variables|Default|SetState (Utilities|Select :Index (Variables|Default|GetState) :NewEnumerator0 "NewEnumerator1" :NewEnumerator1 "NewEnumerator2" :NewEnumerator2 "NewEnumerator3" :NewEnumerator3 "NewEnumerator3")))
      (if (Utilities|Enum|Equal(Enum) _output_get "NewEnumerator2")
        (Development|SetHiddeninGame (Variables|Default|GetSmokes) false true)))))

(event EventBeginPlay
  (|CallParentFunction)
  (bind _returnvalue (Rendering|Material|CreateDynamicMaterialInstance (Variables|Default|GetStaticMesh) 0 "/Game/PitaSimulator/Blueprints/Pita/MI_PitaMaterial.MI_PitaMaterial" "None" :!class /Script/Engine.PrimitiveComponent))
  (Variables|Default|SetPitaMaterialInstance _returnvalue)
  (Development|SetHiddeninGame (Variables|Default|GetSmokes) true true))

(event Collision|EventActorBeginOverlap
  (params (OtherActor :type Actor%20Object%20Reference))
  (|CallParentFunction OtherActor) ; This node is disabled and will not be called.\nDrag off pins to build functionality.
)

(event EventTick
  (params (DeltaSeconds :type Float%20%28single-precision%29))
  (|CallParentFunction DeltaSeconds)
  (Rendering|Components|TextRender|SetText (Variables|Default|GetTextRender) (Utilities|Text|ToText(String) (Utilities|String|EnumtoString (Variables|Default|GetState)))))

(fn ConstructionScript
  (|CallParentFunction))