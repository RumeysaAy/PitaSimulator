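; BP_Market is a shop actor where grabbed ingredients form an order that restocks the game's stock actors.
; It binds to child BP_Stock_Market grab events, tallying each ingredient in a map, adding a flat price, and showing the list and total on a TextRender.
; The button checks game mode money against the total, passes quantities to every BP_Stock_Base by ingredient type, then clears the map.
; Purchasing neither deducts money nor resets the total here.
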(event Custom|OnItemGrabbed_Event
  (params (EIngredient :type EIngredients%20Enum :default "NewEnumerator0"))
  (bind _marketlist (Variables|Default|GetMarketList))
  (bind (_value _returnvalue) (Utilities|Map|Find _marketlist EIngredient))
  (Variables|Default|SetTotalPrice (+ (Variables|Default|GetTotalPrice) 2))
  (if _returnvalue
    (Utilities|Map|Add _marketlist EIngredient (+ _value 1))
    (else
      (Utilities|Map|Add _marketlist EIngredient 1)))
  (bind _keys (Utilities|Map|Keys (Variables|Default|GetMarketList)))
  (Variables|Default|SetMarketListString "")
  (for _array_element _keys
    (Variables|Default|SetMarketListString (Utilities|String|Append (Variables|Default|GetMarketListString) (Utilities|String|EnumtoString _array_element) " " (Utilities|String|ToString(Integer) (.Value (Utilities|Map|Find (Variables|Default|GetMarketList) _array_element))) "
")))
  (Rendering|Components|TextRender|SetText (Variables|Default|GetTextRender) (Utilities|Text|ToText(String) (Utilities|String|Append (Variables|Default|GetMarketListString) "Total Price: " (Utilities|String|ToString(Integer) (Variables|Default|GetTotalPrice))))))

(event Custom|OnButtonInteraction_Event
  (params (ButtonState :type EButtonState%20Enum :default "NewEnumerator0"))
  (bind _money (Class|BPIEconomy|GetCurrentMoney(Message) (Game|GetGameMode)))
  (if (>= _money (Variables|Default|GetTotalPrice))
    (bind _outactors (Actor|GetAllActorsOfClass "/Game/PitaSimulator/Blueprints/Stock/BP_Stock_Base.BP_Stock_Base_C"))
    (for _array_element _outactors
      (Default|ChangeStock _array_element (.Value (Utilities|Map|Find (Variables|Default|GetMarketList) (Variables|/Game/PitaSimulator/Blueprints/Stock/BP_Stock_Base.BP_Stock_Base_C|GetIngredientType _array_element)))))
    (Utilities|Map|Clear (Variables|Default|GetMarketList))))

(event EventBeginPlay
  (Utilities|FlowControl|Sequence
    (:then_0
      (for _array_element (Components|GetChildrenComponents (Variables|Default|GetStaticMesh) false)
        (bind _aschild_actor_component (Utilities|Casting|CastToChildActorComponent _array_element))
        (bind _asbp_stock_market (Utilities|Casting|CastToBP_Stock_Market (Variables|/Script/Engine.ChildActorComponent|GetChildActor _aschild_actor_component)))
        (EventDispatchers|AssignOnItemGrabbed _asbp_stock_market (delegate Custom|OnItemGrabbed_Event))))
    (:then_1
      (bind _asbp_button_base (Utilities|Casting|CastToBP_Button_Base (Variables|/Script/Engine.ChildActorComponent|GetChildActor (Variables|Default|GetButton))))
      (EventDispatchers|AssignOnButtonInteraction _asbp_button_base (delegate Custom|OnButtonInteraction_Event)))))

(event Collision|EventActorBeginOverlap
  (params (OtherActor :type Actor%20Object%20Reference)))

(event EventTick
  (params (DeltaSeconds :type Float%20%28single-precision%29)))

(fn ConstructionScript)