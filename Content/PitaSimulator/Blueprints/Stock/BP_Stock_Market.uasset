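; BP_Stock_Market is an interactable stock point in Pita Simulator that holds a count of one ingredient type.
; Interacting empty-handed takes one if any remain, firing OnItemGrabbed with the type; holding a matching ingredient destroys it and returns one to stock.
; ChangeStock updates the count and its TextRender label.
; The construction script picks the static mesh from IngredientType, so each placed instance previews its ingredient.
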(event OnInteractStart(BP_InteractableComponent)
  (bind (_grabbed _grabbedactor) (Class|BPIInteractionSystem|GetGrabbedItem(Message) (Game|GetPlayerController 0)))
  (if _grabbed
    (bind _asbp_ingredient_base (Utilities|Casting|CastToBP_Ingredient_Base _grabbedactor))
    (Variables|Default|SetAs%20BP%20Ingredient%20Base _asbp_ingredient_base)
    (if (Utilities|Enum|Equal(Enum) (Variables|/Game/PitaSimulator/Blueprints/Ingredients/BP_Ingredient_Base.BP_Ingredient_Base_C|GetIngredientType _asbp_ingredient_base) (Variables|Default|GetIngredientType))
      (Class|BPIInteractionSystem|DropAnyItem(Message) (Game|GetPlayerController 0))
      (Actor|DestroyActor (Variables|Default|GetAs%20BP%20Ingredient%20Base))
      (CallFunction|ChangeStock 1))
    (elif (> (Variables|Default|GetCount) 0)
      (Default|CallOnItemGrabbed (Variables|Default|GetIngredientType))
      (CallFunction|ChangeStock -1))))

(event Custom|ChangeStock
  (params (Value :type Integer))
  (Variables|Default|SetCount (+ (Variables|Default|GetCount) Value))
  (Rendering|Components|TextRender|SetText (Variables|Default|GetTextRender) (Utilities|Text|ToText(Integer) (Variables|Default|GetCount))))

(event EventBeginPlay
  (|CallParentFunction)
  (Rendering|Components|TextRender|SetText (Variables|Default|GetTextRender) (Utilities|Text|ToText(Integer) (Variables|Default|GetCount))))

(event Collision|EventActorBeginOverlap
  (params (OtherActor :type Actor%20Object%20Reference))
  (|CallParentFunction OtherActor) ; This node is disabled and will not be called.\nDrag off pins to build functionality.
)

(event EventTick
  (params (DeltaSeconds :type Float%20%28single-precision%29))
  (|CallParentFunction DeltaSeconds) ; This node is disabled and will not be called.\nDrag off pins to build functionality.
)

(fn ConstructionScript
  (|CallParentFunction)
  (Components|StaticMesh|SetStaticMesh (Variables|Default|GetStaticMesh) (Utilities|Select :Index (Variables|Default|GetIngredientType) :NewEnumerator0 "/Game/Fab/Flour_bag/sm_flourbag.sm_flourbag" :NewEnumerator1 "/Game/Fab/Water_Bottle_Free/Bottle_Water_perfect.Bottle_Water_perfect" :NewEnumerator2 "/Game/Fab/Soybean/soybean.soybean" :NewEnumerator3 "/Game/Fab/Yogurt/yeast_maya.yeast_maya")))