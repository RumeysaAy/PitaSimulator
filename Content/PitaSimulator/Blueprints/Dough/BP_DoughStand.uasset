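; Dough stand where ingredients are attached and counted against a recipe, producing a dough once the counts match.
; Attachment is allowed only while that ingredient type is below its recipe count; each addition destroys the ingredient and scales the Bread placeholder by attached count.
; On completion it hides Bread, spawns BP_Dough with a reference to itself, and disables box collision.
; UnlockSlot clears the slot, restores query collision and resets the count map.
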(event EventBeginPlay
  (|CallParentFunction) ; This node is disabled and will not be called.\nDrag off pins to build functionality.
)

(event Collision|EventActorBeginOverlap
  (params (OtherActor :type Actor%20Object%20Reference))
  (|CallParentFunction OtherActor) ; This node is disabled and will not be called.\nDrag off pins to build functionality.
)

(event EventTick
  (params (DeltaSeconds :type Float%20%28single-precision%29))
  (|CallParentFunction DeltaSeconds) ; This node is disabled and will not be called.\nDrag off pins to build functionality.
)

(fn ConstructionScript
  (|CallParentFunction))

(fn FindNewLockStatus
  (bind _currentstatus (Variables|Default|GetCurrentStatus))
  (bind _asbp_ingredient_base (Utilities|Casting|CastToBP_Ingredient_Base (Variables|Default|GetGrabbed%20Actor)))
  (Utilities|Map|Add _currentstatus (Variables|/Game/PitaSimulator/Blueprints/Ingredients/BP_Ingredient_Base.BP_Ingredient_Base_C|GetIngredientType _asbp_ingredient_base) (+ (.Value (Utilities|Map|Find _currentstatus (Variables|/Game/PitaSimulator/Blueprints/Ingredients/BP_Ingredient_Base.BP_Ingredient_Base_C|GetIngredientType _asbp_ingredient_base))) 1))
  (Utilities|FlowControl|Sequence
    (:then_1
      (Transformation|SetWorldScale3D (Variables|Default|Getbread) (* "0.500000,0.500000,0.500000" (Utilities|Array|Length (Variables|Default|GetAttachedActors))))
      (Actor|DestroyActor (Variables|Default|GetGrabbed%20Actor))
      (bind _success (CallFunction|IngredientReady?))
      (bind _output_get (Variables|Default|SetLocked? _success))
      (if _output_get
        (Transformation|SetWorldScale3D (Variables|Default|Getbread) "0, 0, 0")
        (Utilities|Array|Clear (Variables|Default|GetAttachedActors))
        (Game|SpawnActorfromClass "/Game/PitaSimulator/Blueprints/Dough/BP_Dough.BP_Dough_C" (Transformation|GetWorldTransform (Variables|Default|GetDoughSpawnLocation)) "AlwaysSpawn" "MultiplyWithRoot" 0 self 0)
        (Collision|SetCollisionEnabled (Variables|Default|GetBox) "NoCollision")))))

(fn CheckAttachable?
  (params (A :type Boolean) (Object :type Object%20Object%20Reference))
  (if (|CallParentFunction A Object)
    (bind _asbp_ingredient_base (Utilities|Casting|CastToBP_Ingredient_Base Object)
      (:then
        (return (< (.Value (Utilities|Map|Find (Variables|Default|GetCurrentStatus) (Variables|/Game/PitaSimulator/Blueprints/Ingredients/BP_Ingredient_Base.BP_Ingredient_Base_C|GetIngredientType _asbp_ingredient_base))) (.Value (Utilities|Map|Find (Variables|Default|GetRecipe) (Variables|/Game/PitaSimulator/Blueprints/Ingredients/BP_Ingredient_Base.BP_Ingredient_Base_C|GetIngredientType _asbp_ingredient_base))))))
      (:CastFailed
        (return false)))
    (else
      (return false))))

(fn IngredientReady?
  (bind _keys (Utilities|Map|Keys (Variables|Default|GetRecipe)))
  (bind _array_element (Utilities|Array|ForEachLoopwithBreak _keys)
    (:LoopBody
      (Development|PrintString (Utilities|String|Append (Utilities|String|EnumtoString _array_element) " Current: " (Utilities|String|ToString(Integer) (.Value (Utilities|Map|Find (Variables|Default|GetCurrentStatus) _array_element))) " Recipe: " (Utilities|String|ToString(Integer) (.Value (Utilities|Map|Find (Variables|Default|GetRecipe) _array_element)))))
      (if (!= (.Value (Utilities|Map|Find (Variables|Default|GetCurrentStatus) _array_element)) (.Value (Utilities|Map|Find (Variables|Default|GetRecipe) _array_element)))
        (return false)))
    (:Completed
      (return true))))

(fn UnlockSlot
  (params (DestroyedActor :type Actor%20Object%20Reference))
  (CallFunction|ClearSlot)
  (Collision|SetCollisionEnabled (Variables|Default|GetBox) "QueryOnly")
  (Variables|Default|SetCurrentStatus (Utilities|Map|MakeMap "NewEnumerator0" 0)))