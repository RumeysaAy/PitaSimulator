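; BP_Dough is an interactable dough actor that progresses through Unkneaded, Kneaded, Rested and Ready states to become a pita.
; Completed interactions on its BP_InteractableComponent advance the state, and a timer also moves Kneaded dough to Rested.
; ChangeState swaps meshes and retunes the interaction per stage, then replaces the actor with BP_Pita at Ready.
; Tick writes the current state and progress to a TextRender.
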(event OnInteractionCompleted(BP_InteractableComponent)
  (CallFunction|ChangeState (Utilities|Select :Index (Variables|Default|GetState) :NewEnumerator0 "NewEnumerator1" :NewEnumerator1 "NewEnumerator2" :NewEnumerator2 "NewEnumerator3" :NewEnumerator3 "NewEnumerator3")))

(event EventBeginPlay
  (|CallParentFunction)
  (Variables|/Game/PitaSimulator/InteractionSystem/BP_InteractableComponent.BP_InteractableComponent_C|SetInteractionDuration (Variables|Default|GetBP_InteractableComponent) (Variables|Default|GetKneadDuration)))

(event Collision|EventActorBeginOverlap
  (params (OtherActor :type Actor%20Object%20Reference))
  (|CallParentFunction OtherActor) ; This node is disabled and will not be called.\nDrag off pins to build functionality.
)

(event EventTick
  (params (DeltaSeconds :type Float%20%28single-precision%29))
  (|CallParentFunction DeltaSeconds)
  (Rendering|Components|TextRender|SetText (Variables|Default|GetTextRender) (Utilities|Text|ToText(String) (Utilities|String|Append "Current State: " (Utilities|String|EnumtoString (Variables|Default|GetState)) "
Progress: " (Utilities|String|ToString(Text) (Utilities|Text|ToText(Float) (Variables|Default|GetProgress) "HalfToEven"))))))

(fn ConstructionScript
  (|CallParentFunction))

(fn ChangeState
  (params (NewState :type EDoughStates%20Enum :default "NewEnumerator0"))
  (bind _bp_interactablecomponent (Variables|Default|GetBP_InteractableComponent))
  (Variables|Default|SetState NewState)
  (switch Utilities|FlowControl|Switch|SwitchonEDoughStates NewState
    (:NewEnumerator1
      (Variables|Default|SetProgress 0.0)
      (Variables|Default|SetState "NewEnumerator1")
      (Components|StaticMesh|SetStaticMesh (Variables|Default|GetStaticMesh) "/Game/PitaSimulator/Blueprints/Dough/SM_Dough_Kneaded.SM_Dough_Kneaded")
      (Variables|/Game/PitaSimulator/InteractionSystem/BP_InteractableComponent.BP_InteractableComponent_C|SetInteractionDuration (Variables|Default|GetBP_InteractableComponent) 0.0)
      (Utilities|Time|SetTimerbyFunctionName 0 "Rest" (Variables|Default|GetRestDuration)))
    (:NewEnumerator2
      (Components|StaticMesh|SetStaticMesh (Variables|Default|GetStaticMesh) "/Game/PitaSimulator/Blueprints/Dough/SM_Dough_Rested.SM_Dough_Rested")
      (Variables|/Game/PitaSimulator/InteractionSystem/BP_InteractableComponent.BP_InteractableComponent_C|SetInteractionType _bp_interactablecomponent "NewEnumerator4")
      (Variables|/Game/PitaSimulator/InteractionSystem/BP_InteractableComponent.BP_InteractableComponent_C|SetInteractionDuration _bp_interactablecomponent (Variables|Default|GetReadyDuration)))
    (:NewEnumerator3
      (Actor|DestroyActor)
      (Game|SpawnActorfromClass "/Game/PitaSimulator/Blueprints/Pita/BP_Pita.BP_Pita_C" (Transformation|GetActorTransform) "AlwaysSpawn" "MultiplyWithRoot" 0 0))))

(fn Rest
  (CallFunction|ChangeState "NewEnumerator2"))